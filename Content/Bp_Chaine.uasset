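; Chain actor that lays copies of a link mesh (Maillon) along a spline, with no active gameplay logic.
; The construction script rebuilds a hierarchical instanced static mesh, spacing links by MaillonSize and deriving their count from spline length divided by MaillonSize minus one.
; Each link follows the spline's local position and rotation, with a FlipFlop alternating an extra 90-degree roll to interlock neighbors.
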(fn `UserConstructionScript`
  (`InstancedStaticMeshComponent.ClearInstances` (`self.HierarchicalInstancedStaticMesh`))
  (`StaticMeshComponent.SetStaticMesh` (`self.HierarchicalInstancedStaticMesh`) (`self.Maillon`))
  (for _index (range (`KismetMathLibrary.FTrunc` (/ (`SplineComponent.GetSplineLength` (`self.Spline`)) (- (`self.MaillonSize`) 1.0))))
    (`/Engine/EditorBlueprintResources/StandardMacros.FlipFlop`
      (:`A`
        (set `self.TargetRot` 0.0))
      (:`B`
        (set `self.TargetRot` 90.0)))
    (bind _returnvalue (`SplineComponent.GetTransformAtDistanceAlongSpline` (`self.Spline`) (* _index (`self.MaillonSize`)) "Local" false))
    (`InstancedStaticMeshComponent.AddInstance` (`self.HierarchicalInstancedStaticMesh`) (`KismetMathLibrary.MakeTransform` (.location _returnvalue) (`KismetMathLibrary.MakeRotator` (+ (.roll (.rotation _returnvalue)) (`self.TargetRot`)) (.pitch (.rotation _returnvalue)) (.yaw (.rotation _returnvalue)))) false)))